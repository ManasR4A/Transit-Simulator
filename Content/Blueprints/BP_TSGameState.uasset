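; Game state for a city simulation that caches level buildings, bus stops and the nav mesh, then tells the bus tracking system to spawn buses.
; Commercial buildings are queued through AddRequestingComm and processed on a looping timer.
; For each missing Sim, random residential buildings attempt spawns toward the requester, retrying under a shared try counter that is never reset.
; Industrial request processing is an empty stub.
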(event `self.ReceiveBeginPlay`
  ;[1 1 1] Getting references to all the buildings in the level
  (bind _returnvalue (`GameplayStatics.GetActorOfClass` "/Script/NavigationSystem.NavMeshBoundsVolume"))
  (set `self.Nav Mesh` _returnvalue)
  (bind _returnvalue_2 (`GameplayStatics.GetActorOfClass` "/Game/Blueprints/AI/Bus/BP_BusTrackingSystem.BP_BusTrackingSystem_C"))
  (set `self.Bus Tracking Manager Ref` _returnvalue_2)
  (bind _outactors (`GameplayStatics.GetAllActorsOfClass` "/Game/Blueprints/Infrastructure/Buildings/BP_ResBuilding.BP_ResBuilding_C"))
  (set `self.ResBuildings` _outactors)
  (bind _outactors_2 (`GameplayStatics.GetAllActorsOfClass` "/Game/Blueprints/Infrastructure/Buildings/BP_COmmBuilding.BP_CommBuilding_C"))
  (set `self.CommBuildings` _outactors_2)
  (bind _outactors_3 (`GameplayStatics.GetAllActorsOfClass` "/Game/Blueprints/Infrastructure/Buildings/BP_IndustryBuilding.BP_IndustryBuilding_C"))
  (set `self.Indistrial Buildings` _outactors_3)
  (bind _outactors_4 (`GameplayStatics.GetAllActorsOfClass` "/Game/Blueprints/Infrastructure/Buildings/BP_OfficeBuilding.BP_OfficeBuilding_C"))
  (set `self.OfficeBuildings` _outactors_4)
  (bind _returnvalue_3 (`KismetSystemLibrary.K2_SetTimerDelegate` (delegate `Process Requests`) 5.0 true))
  (set `self.Request Processing Timer` _returnvalue_3)
  (bind _outactors_5 (`GameplayStatics.GetAllActorsOfClass` "/Game/Blueprints/Infrastructure/BP_BusStop.BP_BusStop_C"))
  (set `self.BusStops` _outactors_5)
  (`/Game/Blueprints/AI/Bus/BP_BusTrackingSystem.Spawn Busses` (`self.Bus Tracking Manager Ref`)))

(event `Process Requests`
  (for _array_element (`self.ReqestingCommBuildings`)
    (`self.Process Commercial Request` _array_element))
  (`KismetArrayLibrary.Array_Clear` (`self.ReqestingCommBuildings`)))

(fn `Add Requesting Comm`
  (params (`Requestung Building` :type "/Game/Blueprints/Infrastructure/Buildings/BP_COmmBuilding Object Reference"))
  (returns (bRequestAck :type Boolean))
  (`KismetArrayLibrary.Array_Add` (`self.ReqestingCommBuildings`) `Requestung Building`)
  (return true))

(fn `Get Random Res Building`
  (returns (`Rand Res Building` :type "/Game/Blueprints/Infrastructure/Buildings/BPC_ResBuilding Object Reference"))
  (return (`self.GetComponentByClass` (`|GetArrayItem` (`self.ResBuildings`) (`KismetMathLibrary.RandomIntegerInRange` 0 (- (`KismetArrayLibrary.Array_Length` (`self.ResBuildings`)) 1))) "/Game/Blueprints/Infrastructure/Buildings/BPC_ResBuilding.BPC_ResBuilding_C")))

(fn `Process Commercial Request`
  (params (`Requesting Commercial Building` :type "/Game/Blueprints/Infrastructure/Buildings/BP_COmmBuilding Object Reference"))
  (locals (`Spawn Tries` :type Integer) (`Spawned Sims` :type Integer))
  (bind _returnvalue (`self.GetComponentByClass` `Requesting Commercial Building` "/Game/Blueprints/Infrastructure/Buildings/BPC_CommBuilding.BPC_CommBuilding_C"))
  (set `local.Spawned Sims` 0)
  (for _ (range 1 (+ (- (`/Game/Blueprints/Infrastructure/Buildings/BPC_CommBuilding.Max Sims` _returnvalue) (`/Game/Blueprints/Infrastructure/Buildings/BPC_CommBuilding.Current Sims` _returnvalue)) 1))
    (bind _rand_res_building (`self.Get Random Res Building` :!label _label))
    (bind _spawned_sim (`/Game/Blueprints/Infrastructure/Buildings/BPC_ResBuilding.Try to Spawn Sim` _rand_res_building `Requesting Commercial Building` (`self.Nav Mesh`)))
    (`/Engine/EditorBlueprintResources/StandardMacros.IncrementInt` (`local.Spawn Tries`)
      (:`  `
        (if _spawned_sim
          (`/Engine/EditorBlueprintResources/StandardMacros.IncrementInt` (`local.Spawned Sims`))
          (elif (<= (`local.Spawn Tries`) (`self.Max Spawn Tries`))
            (goto _label)))))))

(fn `Process Industrial Requests`)

(fn `UserConstructionScript`)