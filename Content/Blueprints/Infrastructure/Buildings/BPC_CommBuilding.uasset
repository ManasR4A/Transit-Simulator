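; Commercial building component that tracks a building's sims and goods and requests supply through the game state.
; On BeginPlay it reads sim capacity, then sets the mesh material and a random goods cap by low or high building type.
; A looping timer registers the building with BP_TSGameState while sims are below capacity and no request is pending; the goods check triggers nothing.
; Callbacks clear failed requests and add received amounts.
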(event `self.ReceiveBeginPlay`
  (bind _returnvalue (`Actor.GetComponentByClass` (`self.ParentBuilding`) "/Script/Engine.StaticMeshComponent"))
  ;[1 1 1] Begin Play Initial Setup
  (bind _returnvalue_2 (`KismetSystemLibrary.K2_SetTimerDelegate` (delegate `Check and Request`) (`self.Request Time`) true))
  (set `self.Request Timer` _returnvalue_2)
  (bind _asbp_comm_building (cast `/Game/Blueprints/Infrastructure/Buildings/BP_COmmBuilding` (`self.GetOwner`)))
  (bind _output_get (set `self.ParentBuilding` _asbp_comm_building))
  (bind _asbp_tsgame_state (cast `/Game/Blueprints/BP_TSGameState` (`GameplayStatics.GetGameState`)))
  (set `self.Game State Ref` _asbp_tsgame_state)
  (bind _returnvalue_3 (`Actor.GetComponentByClass` _output_get "/Script/TransitSimulator.TSBuildingComponent"))
  (set `self.Max Sims` (`TSBuildingComponent.SimCapacity` _returnvalue_3))
  (set `self.Current Sims` 0)
  (switch `EBuildingType` (`TSBuildingComponent.BuildingType` _returnvalue_3)
    (:`LowRes`
      (`PrimitiveComponent.SetMaterial` _returnvalue 0 (`self.Material Low`))
      (set `self.Max Goods` (`KismetMathLibrary.RandomIntegerInRange` 10 40)))
    (:`HighRes`
      (`PrimitiveComponent.SetMaterial` _returnvalue 0 (`self.Material High`))
      (set `self.Max Goods` (`KismetMathLibrary.RandomIntegerInRange` 50 100)))))

(event `Check and Request`
  (`|ExecutionSequence`
    (:`then_0`
      ;[1 1 1] Check Good requirement
      (if (< (`self.Current Goods`) (`self.Max Goods`))
        _))
    (:`then_1`
      ;[1 1 1] Check Sim requirements
      (if (and (< (`self.Current Sims`) (`self.Max Sims`)) (not (`self.Requested`)))
        (bind _brequestack (`/Game/Blueprints/BP_TSGameState.Add Requesting Comm` (`self.Game State Ref`) (`self.ParentBuilding`)))
        (set `self.Requested` _brequestack)
        (`KismetSystemLibrary.PrintString` "Commercial sent request" true true (struct :`R` 0.2 :`G` 0.2 :`B` 1.0 :`A` 1.0))))))

(fn `IsRequestProcessed`
  (params (`request Processed` :type Boolean))
  (if (not `request Processed`)
    (set `self.Requested` false)))

(fn `Recieve Requested`
  (params (`Recieved Sims` :type Integer) (`Recieved Goods` :type Integer))
  (set `self.Current Sims` (+ (`self.Current Sims`) `Recieved Sims`))
  (set `self.Current Goods` (+ (`self.Current Goods`) `Recieved Goods`)))