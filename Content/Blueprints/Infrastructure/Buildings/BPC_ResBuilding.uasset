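; BPC_ResBuilding is a residential building component that sets the building's look and supplies pedestrian sims.
; On begin play it takes its sim count from TSBuildingComponent's capacity and applies a low or high residential material by building type.
; TryToSpawnSim spawns a pedestrian at the parent road while sims remain, decrementing the count and starting its trip to the target building's road on a given navmesh.
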(event `self.ReceiveBeginPlay`
  (bind _returnvalue (`Actor.GetComponentByClass` (`self.ParentBuilding`) "/Script/Engine.StaticMeshComponent"))
  ;[1 1 1] Begin Play
  (bind _asbp_res_building (cast `/Game/Blueprints/Infrastructure/Buildings/BP_ResBuilding` (`self.GetOwner`)))
  (bind _output_get (set `self.ParentBuilding` _asbp_res_building))
  (bind _returnvalue_2 (`Actor.GetComponentByClass` _output_get "/Script/TransitSimulator.TSBuildingComponent"))
  (set `self.Current Sims` (`TSBuildingComponent.SimCapacity` _returnvalue_2))
  (switch `EBuildingType` (`TSBuildingComponent.BuildingType` _returnvalue_2)
    (:`LowRes`
      (`PrimitiveComponent.SetMaterial` _returnvalue 0 (`self.Material Low`)))
    (:`HighRes`
      (`PrimitiveComponent.SetMaterial` _returnvalue 0 (`self.Material High`)))))

(event `Spawn Ped`
  (params (Destination :type "Vector Structure") (`Nav Mesh Road` :type "Actor Object Reference"))
  (bind _returnvalue (`Actor.GetTransform` (`/Game/Blueprints/Infrastructure/Buildings/BP_ResBuilding.ParentRoadRef` (`self.ParentBuilding`))))
  ;[1 1 1] Spawn Ped From Residential
  (bind _returnvalue_2 (`|SpawnActorFromClass` "/Game/Blueprints/AI/Ped/BP_PedChar.BP_PedChar_C" (`KismetMathLibrary.MakeTransform` (`KismetMathLibrary.MakeVector` (.x (.location _returnvalue)) (.y (.location _returnvalue)) 50.0) (.rotation _returnvalue) (.scale _returnvalue)) "AdjustIfPossibleButAlwaysSpawn" "OverrideRootScale" null null))
  (`KismetArrayLibrary.Array_AddUnique` (`self.Spawned Peds`) _returnvalue_2)
  (`/Engine/EditorBlueprintResources/StandardMacros.DecrementInt` (`self.Current Sims`)
    (:`  `
      (set `/Game/Blueprints/AI/Ped/BP_PedChar.Parent Building` (`self.ParentBuilding`) _returnvalue_2)
      (set `/Game/Blueprints/AI/Ped/BP_PedChar.Source` (`Actor.K2_GetActorLocation` (`/Game/Blueprints/Infrastructure/Buildings/BP_ResBuilding.ParentRoadRef` (`self.ParentBuilding`))) _returnvalue_2)
      (set `/Game/Blueprints/AI/Ped/BP_PedChar.Destination` Destination _returnvalue_2)
      (set `/Game/Blueprints/AI/Ped/BP_PedChar.NavMeshActor` `Nav Mesh Road` _returnvalue_2)
      (`/Game/Blueprints/AI/Ped/BP_PedChar.Start Simulating` _returnvalue_2))))

(fn `Try to Spawn Sim`
  (params (`Target Building` :type "/Game/Blueprints/Infrastructure/Buildings/BP_COmmBuilding Object Reference") (`Nav Mesh to use` :type "NavMeshBoundsVolume Object Reference"))
  (returns (`Spawned Sim` :type Boolean))
  (if (> (`self.Current Sims`) 0)
    (`self.Spawn Ped` (`Actor.K2_GetActorLocation` (`/Game/Blueprints/Infrastructure/Buildings/BP_COmmBuilding.ParentRoadRef` `Target Building`)) `Nav Mesh to use`)
    (return true)
    (else
      (return false) ; Has No Sims to Spawn
    )))