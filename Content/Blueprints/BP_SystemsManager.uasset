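; BP_SystemsManager evaluates bus travel as an option for pedestrian trips.
; It finds the stops on the bus manager's line nearest the source and destination by synchronous navmesh path length, capped at the total trip length.
; The combined walking distance, as a ratio of the trip length, is looked up in a distance-based probability curve to return a utility plus both stops.
; It also caches the game state on BeginPlay.
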(event `self.ReceiveBeginPlay`
  (bind _asbp_tsgame_state (cast `/Game/Blueprints/BP_TSGameState` (`GameplayStatics.GetGameState`)))
  (set `self.Game State Ref` _asbp_tsgame_state))

(fn `Get Bus Expected Utility`
  (params (`Caller Ped` :type "/Game/Blueprints/AI/Ped/BP_PedChar Object Reference") (`Source Loc` :type "Vector Structure") (`Destination Location` :type "Vector Structure") (`Total Path Len` :type "Float (double-precision)"))
  (returns (`Bus Utility` :type "Float (double-precision)") (`Ret Src Stop` :type "/Game/Blueprints/Infrastructure/BP_BusStop Object Reference") (`Ret Dest Stop` :type "/Game/Blueprints/Infrastructure/BP_BusStop Object Reference"))
  (locals (`Source Stop` :type "/Game/Blueprints/Infrastructure/BP_BusStop Object Reference") (`Destination Stop` :type "/Game/Blueprints/Infrastructure/BP_BusStop Object Reference") (`Walking Distance` :type "Float (double-precision)"))
  ;[1 1 1] Get Source and Destination Bus Stops
  (bind (_closest_stop _distance) (`self.Get Closest Stop` `Source Loc` `Total Path Len`))
  (set `local.Source Stop` _closest_stop)
  (set `local.Walking Distance` _distance)
  (bind (_closest_stop_2 _distance_2) (`self.Get Closest Stop` `Destination Location` `Total Path Len`))
  (set `local.Walking Distance` (+ _distance_2 (`local.Walking Distance`)))
  (set `local.Destination Stop` _closest_stop_2)
  (return (`CurveFloat.GetFloatValue` (`self.Distance Based Probability`) (/ (`local.Walking Distance`) `Total Path Len`)) (`local.Source Stop`) (`local.Destination Stop`)))

(fn `Get Closest Stop`
  (params (`Current Loc` :type "Vector Structure") (`Total Path Len` :type "Float (double-precision)"))
  (returns (`Closest Stop` :type "/Game/Blueprints/Infrastructure/BP_BusStop Object Reference") (Distance :type "Float (double-precision)"))
  (locals (`Shortest path` :type "Float (double-precision)") (`Closest Bus Stop` :type "/Game/Blueprints/Infrastructure/BP_BusStop Object Reference"))
  (set `local.Shortest path` `Total Path Len`)
  (for _array_element (`/Game/Blueprints/AI/Bus/BP_BusLine.Bus Line` (`self.Bus Manager Ref`))
    (bind _returnvalue (`NavigationSystemV1.FindPathToLocationSynchronously` `Current Loc` (`self.K2_GetActorLocation` _array_element) (`self.Nav Mesh Ref`) null))
    (bind _returnvalue_2 (`NavigationPath.GetPathLength` _returnvalue))
    (if (< _returnvalue_2 (`local.Shortest path`))
      (set `local.Shortest path` _returnvalue_2)
      (set `local.Closest Bus Stop` _array_element)))
  (return (`local.Closest Bus Stop`) (`local.Shortest path`)))

(fn `UserConstructionScript`)