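; Bus manager actor that spawns and starts a bus on its BusLine and serves as its route tracker.
; SpawnBusses, intended for the game state to call, places one bus at a random stop, marks it occupied and registers it.
; Stop selection retries up to the game state's MaxSpawnTries but re-rolls the returned index, so occupancy isn't guaranteed.
; GetNextBusStop supplies the following stop, wrapping to the first.
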(event `self.ReceiveBeginPlay`
  ;[1 1 1] Initialization
  (bind _asbp_tsgame_state (cast `/Game/Blueprints/BP_TSGameState` (`GameplayStatics.GetGameState`))
    (:`then`
      (bind _output_get (set `self.Game State Ref` _asbp_tsgame_state))
      (set `self.Spawn Tries` (`/Game/Blueprints/BP_TSGameState.Max Spawn Tries` _output_get)))
    (:`CastFailed`
      (`KismetSystemLibrary.PrintString` "Game State Cast Failed" true true (struct :`R` 1.0 :`A` 1.0)))))

(event `Spawn Busses`
  ;[1 1 1] Spawning Initial busses. To be called by game state
  (for _ (range 1)
    (bind _random_bus_stop (`self.Get Random Unoccupied Bus Stop`))
    (bind _returnvalue (`self.GetTransform` _random_bus_stop))
    (`KismetSystemLibrary.PrintString` (`KismetStringLibrary.Conv_TransformToString` _returnvalue))
    (bind _returnvalue_2 (`|SpawnActorFromClass` "/Game/Blueprints/AI/Bus/BP_BusChar.BP_BusChar_C" (`KismetMathLibrary.MakeTransform` (`KismetMathLibrary.MakeVector` (.x (.location _returnvalue)) (.y (.location _returnvalue)) 50.0) (`KismetMathLibrary.MakeRotator` (.roll (.rotation _returnvalue)) (.pitch (.rotation _returnvalue)) (+ (.yaw (.rotation _returnvalue)) 90.0)) (.scale _returnvalue)) "AdjustIfPossibleButAlwaysSpawn" "OverrideRootScale" null null))
    (set `/Game/Blueprints/AI/Bus/BP_BusChar.Bus Tracker Ref` self _returnvalue_2)
    (set `/Game/Blueprints/Infrastructure/BP_BusStop.isOccupied` true _random_bus_stop)
    (`KismetArrayLibrary.Array_Add` (`self.Active Busses`) _returnvalue_2))
  (`KismetSystemLibrary.PrintString` (`KismetStringLibrary.Concat_StrStr` "Bus Spawned = " (`KismetStringLibrary.Conv_IntToString` (`KismetArrayLibrary.Array_Length` (`self.Active Busses`)))) true true (struct :`R` 1.0 :`G` 1.0 :`A` 1.0))
  (for _array_element (`self.Active Busses`)
    (`/Game/Blueprints/AI/Bus/BP_BusChar.Start Bus` _array_element))
  (`KismetSystemLibrary.PrintString` "Started All Busses" true true (struct :`R` 1.0 :`G` 1.0 :`A` 1.0)))

(fn `Get Next Bus Stop`
  (params (`Requesting Bus` :type "/Game/Blueprints/AI/Bus/BP_BusChar Object Reference"))
  (returns (`Next Stop` :type "/Game/Blueprints/Infrastructure/BP_BusStop Object Reference"))
  (bind _bus_line (`self.Bus Line`))
  (bind _returnvalue (`KismetArrayLibrary.Array_Find` _bus_line (`/Game/Blueprints/AI/Bus/BP_BusChar.Next Stop` `Requesting Bus`)))
  (if (!= (- (`KismetArrayLibrary.Array_Length` _bus_line) 1) _returnvalue)
    (return (`|GetArrayItem` (`self.Bus Line`) (+ _returnvalue 1)))
    (else
      (return (`|GetArrayItem` (`self.Bus Line`))))))

(fn `Get Random Unoccupied Bus Stop`
  (returns (`Random Bus Stop` :type "/Game/Blueprints/Infrastructure/BP_BusStop Object Reference"))
  (bind _bus_line (`self.Bus Line`))
  (bind _output (`|GetArrayItem` _bus_line (`KismetMathLibrary.RandomIntegerInRange` 0 (- (`KismetArrayLibrary.Array_Length` _bus_line) 1))))
  (for _ (range 1 (+ (`self.Spawn Tries`) 1))
    (if (not (`/Game/Blueprints/Infrastructure/BP_BusStop.isOccupied` _output))
      (return _output))))

(fn `UserConstructionScript`)